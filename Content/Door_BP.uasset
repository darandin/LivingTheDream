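; Door Blueprint that swings open when something enters its trigger Box and closes once no player character remains inside.
; Box begin overlap calls Open, which plays a timeline that drives the Door's relative yaw.
; Box end overlap queries for overlapping TopDownCharacter pawns and calls Close, which reverses the same timeline, when none are found.
; An IsOpen flag keeps repeated overlaps from retriggering either motion.
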(event `Open`
  (if (not (`self.IsOpen?`))
    (set `self.IsOpen?` true)
    (bind (_direction _newtrack_0) (`Timeline|Timeline_0` :!label _label)
      (:`Update`
        (`SceneComponent.K2_SetRelativeRotation` (`self.Door`) (`KismetMathLibrary.MakeRotator` 0.0 0.0 _newtrack_0) false false)))))

(event `self.Box.OnComponentBeginOverlap`
  (params (OverlappedComponent :type "PrimitiveComponent Object Reference") (OtherActor :type "Actor Object Reference") (OtherComp :type "PrimitiveComponent Object Reference") (OtherBodyIndex :type Integer) (bFromSweep :type Boolean) (SweepResult :type "HitResult Structure (by ref)"))
  (`self.Open`))

(event `Close`
  (if (`self.IsOpen?`)
    (set `self.IsOpen?` false)
    (goto _label :!via `Reverse`)))

(event `self.Box.OnComponentEndOverlap`
  (params (OverlappedComponent :type "PrimitiveComponent Object Reference") (OtherActor :type "Actor Object Reference") (OtherComp :type "PrimitiveComponent Object Reference") (OtherBodyIndex :type Integer))
  (bind _box (`self.Box`))
  (bind (_outactors _returnvalue) (`KismetSystemLibrary.ComponentOverlapActors` _box (`KismetMathLibrary.MakeTransform` (`SceneComponent.K2_GetComponentLocation` _box)) (`|MakeArray` "ObjectTypeQuery3" :!type "EObjectTypeQuery Enum") "/Game/TopDownBP/Blueprints/TopDownCharacter.TopDownCharacter_C"))
  (if (not _returnvalue)
    (`self.Close`)))

(fn `UserConstructionScript`)