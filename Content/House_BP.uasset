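; House Blueprint for a top-down game that hides its roof while the local player's character is inside.
; The Roof_trigger component's begin and end overlap events toggle the visibility of the HouseRoof component, without propagating to children.
; Both events act only when the overlapping TopDownCharacter is controlled by player controller 0, so other characters do not affect the roof.
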(event `self.roof_trigger.OnComponentBeginOverlap`
  (params (OverlappedComponent :type "PrimitiveComponent Object Reference") (OtherActor :type "Actor Object Reference") (OtherComp :type "PrimitiveComponent Object Reference") (OtherBodyIndex :type Integer) (bFromSweep :type Boolean) (SweepResult :type "HitResult Structure (by ref)"))
  (bind _astop_down_character (cast `/Game/TopDownBP/Blueprints/TopDownCharacter` OtherActor))
  (if (== (`GameplayStatics.GetPlayerController` 0) (`Pawn.GetController` _astop_down_character))
    (`SceneComponent.SetVisibility` (`self.house_roof`) false false)))

(event `self.roof_trigger.OnComponentEndOverlap`
  (params (OverlappedComponent :type "PrimitiveComponent Object Reference") (OtherActor :type "Actor Object Reference") (OtherComp :type "PrimitiveComponent Object Reference") (OtherBodyIndex :type Integer))
  (bind _astop_down_character (cast `/Game/TopDownBP/Blueprints/TopDownCharacter` OtherActor))
  (if (== (`GameplayStatics.GetPlayerController` 0) (`Pawn.GetController` _astop_down_character))
    (`SceneComponent.SetVisibility` (`self.house_roof`) true false)))

(fn `UserConstructionScript`)